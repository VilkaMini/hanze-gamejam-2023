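; BP_Projectile is a paintball-style projectile that passes its color to what it hits.
; The Construction Script picks one of seven rainbow materials at random, saves it and applies it to the Projectile component.
; On component hit, it sets that saved material on the first slot of the other actor's StaticMeshComponent, if one exists, then destroys itself.
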(event `self.Projectile.OnComponentHit`
  (params (HitComponent :type "PrimitiveComponent Object Reference") (OtherActor :type "Actor Object Reference") (OtherComp :type "PrimitiveComponent Object Reference") (NormalImpulse :type "Vector Structure") (Hit :type "HitResult Structure (by ref)"))
  (bind _returnvalue (`self.GetComponentByClass` OtherActor "/Script/Engine.StaticMeshComponent"))
  ;[1 1 1] Change StaticMesh Color and delete projectile
  (if (`KismetSystemLibrary.IsValid` _returnvalue)
    (`PrimitiveComponent.SetMaterial` _returnvalue 0 (`self.SavedMat`)))
  (`self.K2_DestroyActor`))

(fn `UserConstructionScript`
  (bind _output_get (set `self.SavedMat` (select `int` (`KismetMathLibrary.RandomInteger` 7) :`0` (`self.RedMat`) :`1` (`self.OrangeMat`) :`2` (`self.YellowMat`) :`3` (`self.GreenMat`) :`4` (`self.BlueMat`) :`5` (`self.IndigoMat`) :`6` (`self.VioletMat`))))
  (`PrimitiveComponent.SetMaterial` (`self.Projectile`) 0 _output_get))